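; BP_Door is an interactable door that swings open or closed each time its Interact event fires.
; Interact toggles IsOpen and plays or reverses a timeline whose Alpha, scaled by MaxAngle, sets the door mesh's yaw.
; When the timeline finishes, collision is disabled if the door is open and restored if closed.
; Cursor-over events on the collision component and actor only print placeholder debug strings.
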(event `/Game/Enemies/BPI_Interact.Interact`
  (bind _collision (`self.Collision`))
  (bind _output_get (set `self.IsOpen` (not (`self.IsOpen`))))
  (if _output_get
    (bind (_direction _alpha) (`Timeline|Door Timeline` :!label _label)
      (:`Update`
        (`SceneComponent.K2_SetRelativeRotation` (`self.SM_Door`) (`KismetMathLibrary.MakeRotator` 0.0 0.0 (* _alpha (`self.MaxAngle`))) false false))
      (:`Finished`
        (if (`self.IsOpen`)
          (`PrimitiveComponent.SetCollisionEnabled` _collision "NoCollision")
          (else
            (`PrimitiveComponent.SetCollisionEnabled` _collision "QueryAndPhysics")))))
    (else
      (goto _label :!via `Reverse`))))

(event `self.Collision.OnBeginCursorOver`
  (params (TouchedComponent :type "PrimitiveComponent Object Reference"))
  (`KismetSystemLibrary.PrintString` "Hello"))

(event `self.ReceiveActorEndCursorOver`
  (`KismetSystemLibrary.PrintString` "asdasd"))

(fn `UserConstructionScript`)